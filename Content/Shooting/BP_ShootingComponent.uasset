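; Shooting component that lets its owning actor fire a spread or set of projectiles with a cooldown between shots.
; Shoot spawns the projectile class at every owner ArrowComponent tagged "ShootingArrow", so the arrows define each muzzle position and direction.
; It plays the Escopeta sound at world origin and decrements Ammo on a BP_Cowboy owner, without checking the count.
; A DoOnce gate, reset after a delay, enforces the cooldown.
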(event `Shoot`
  (`/Engine/EditorBlueprintResources/StandardMacros.DoOnce` false :!label _label
    (:`Completed`
      (`|ExecutionSequence`
        (:`then_0`
          (for _array_element (`Actor.GetComponentsByTag` (`self.GetOwner`) "/Script/Engine.ActorComponent" "ShootingArrow")
            (bind _asarrow_component (cast `ArrowComponent` _array_element))
            (`|SpawnActorFromClass` (`self.ProjectileClass`) (`SceneComponent.K2_GetComponentToWorld` _asarrow_component) "Undefined" "OverrideRootScale" null null)))
        (:`then_1`
          (`GameplayStatics.PlaySoundAtLocation` "/Game/Sounds/escopeta.escopeta" (0.0 0.0 0.0) (struct) 1.0 1.0 0.0 null null null))
        (:`then_2`
          (bind _asbp_cowboy (cast `/Game/Cowboy/BP_Cowboy` (`self.GetOwner`)))
          (`/Engine/EditorBlueprintResources/StandardMacros.DecrementInt` (`/Game/Cowboy/BP_Cowboy.Ammo` _asbp_cowboy)))
        (:`then_3`
          (`KismetSystemLibrary.Delay` (`self.ShootingCooldown`))
          (goto _label :!via `Reset`))))))