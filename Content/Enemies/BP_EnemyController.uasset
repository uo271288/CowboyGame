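; AI controller for enemies that chases the cowboy player and keeps the enemy pawn facing them.
; BeginPlay caches the BP_Cowboy actor, and possessing a pawn triggers FollowPlayer, which issues a single AI Move To toward that actor with zero acceptance radius.
; Every tick, while the cached cowboy is valid, it snaps the pawn's rotation to the look-at yaw toward the player.
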(event `self.ReceiveBeginPlay`
  (bind _returnvalue (`GameplayStatics.GetActorOfClass` "/Game/Cowboy/BP_Cowboy.BP_Cowboy_C"))
  (set `self.Cowboy Player` _returnvalue))

(event `FollowPlayer`
  (`|AIMoveTo` null (0.0 0.0 0.0) (`self.Cowboy Player`) 0.0))

(event `self.ReceiveTick`
  (params (DeltaSeconds :type "Float (single-precision)"))
  (bind _returnvalue (`self.K2_GetPawn`))
  (bind _cowboy_player (`self.Cowboy Player`)
    (:`then`
      (bind (_returnvalue_roll _returnvalue_pitch _returnvalue_yaw) (`KismetMathLibrary.BreakRotator` (`KismetMathLibrary.FindLookAtRotation` (`self.K2_GetActorLocation` _returnvalue) (`self.K2_GetActorLocation` _cowboy_player))))
      (`self.K2_SetActorRotation` _returnvalue (`KismetMathLibrary.MakeRotator` 0.0 0.0 _returnvalue_yaw) false))
    (:`else`)))

(event `self.ReceivePossess`
  (params (PossessedPawn :type "Pawn Object Reference"))
  (`self.FollowPlayer`))

(fn `UserConstructionScript`)