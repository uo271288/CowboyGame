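; Enemy spawner that repeatedly spawns enemies at random spots within its Box area from BeginPlay onward.
; GenerateEnemy spawns EnemyClass at a random X and Y inside the box extents, keeping the spawner's Z, then calls itself again after an EnemyTime delay.
; Each cycle randomly picks BP_Cactus or BP_Itachi after spawning, so the choice applies to the next spawn and the first uses the initial EnemyClass.
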(event `self.ReceiveBeginPlay`
  (`self.GenerateEnemy`))

(event `GenerateEnemy`
  (bind _returnvalue (`self.K2_GetActorLocation`))
  (bind (_returnvalue_x _returnvalue_y) (`KismetMathLibrary.BreakVector` (`KismetMathLibrary.RandomPointInBoundingBox` _returnvalue (`BoxComponent.GetScaledBoxExtent` (`self.Box`)))))
  (`|ExecutionSequence`
    (:`then_0`
      (`|SpawnActorFromClass` (`self.Enemy Class`) (`KismetMathLibrary.MakeTransform` (`KismetMathLibrary.MakeVector` _returnvalue_x _returnvalue_y (.z _returnvalue))) "Undefined" "OverrideRootScale" null null))
    (:`then_1`
      (`KismetSystemLibrary.Delay` (`self.EnemyTime`))
      (`self.GenerateEnemy`))
    (:`then_2`
      (if (`KismetMathLibrary.RandomBool`)
        (set `self.Enemy Class` "/Game/Enemies/BP_Cactus.BP_Cactus_C")
        (else
          (set `self.Enemy Class` "/Game/Enemies/BP_Itachi.BP_Itachi_C"))))))

(fn `UserConstructionScript`)